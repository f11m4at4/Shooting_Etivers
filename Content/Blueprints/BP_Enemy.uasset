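; Enemy actor that flies in a straight line and explodes on contact.
; On BeginPlay it finds BP_Player and FindDirection randomly picks a fixed heading: usually straight down, otherwise toward the player's position at that moment.
; Tick moves it along that heading by Speed and delta time, without sweep.
; A Body overlap destroys both the other actor and itself, with an explosion sound and particle effect.
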(event OnComponentBeginOverlap(Body)
  (params (OverlappedComponent :type Primitive%20Component%20Object%20Reference) (OtherActor :type Actor%20Object%20Reference) (OtherComp :type Primitive%20Component%20Object%20Reference) (OtherBodyIndex :type Integer) (bFromSweep :type Boolean) (SweepResult :type Hit%20Result%20Structure%20%28by%20ref%29))
  (Actor|DestroyActor OtherActor)
  (Actor|DestroyActor)
  (Audio|PlaySound2D "/Game/폭팔음_와장창.폭팔음_와장창" 1.0 1.0 0.0 0 0)
  (Effects|SpawnEmitteratLocation "/Game/StarterContent/Particles/P_Explosion.P_Explosion" (Transformation|GetActorLocation)))

(event EventBeginPlay
  (bind _returnvalue (Actor|GetActorOfClass "/Game/Blueprints/BP_Player.BP_Player_C"))
  (Variables|Default|SetTarget _returnvalue)
  (CallFunction|FindDirection))

(event EventTick
  (params (DeltaSeconds :type Float%20%28single-precision%29))
  ;[0.15 0.15 0.15 0.5] 이동하고 싶다.
  (Transformation|SetActorLocation (+ (* DeltaSeconds (* (Variables|Default|GetDirection) (Variables|Default|GetSpeed))) (Transformation|GetActorLocation)) false false))

(fn ConstructionScript)

(fn FindDirection
  (if (> (Math|Random|RandomIntegerinRange 1 10) 3)
    ;[0.15 0.15 0.15 0.5] 아래로 방향구하기
    (Variables|Default|SetDirection "0.000000,0.000000,-1.000000")
    (else
      ;[0.15 0.15 0.15 0.5] 타겟쪽으로 방향을 구하기
      (Variables|Default|SetDirection (Math|Vector|Normalize (- (Transformation|GetActorLocation (Variables|Default|GetTarget)) (Transformation|GetActorLocation)))))))