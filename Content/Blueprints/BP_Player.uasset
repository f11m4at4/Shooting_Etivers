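; BP_Player is a player actor that moves in the Y-Z plane and fires bullets from two gun points.
; The Horizontal and Vertical axis inputs set Direction, which Move applies each Tick with Speed and delta time, without sweep.
; While Fire is held, a Tick timer calls YogaFire for both points at the CreateTime interval, spawning BP_Bullet with a gun sound.
; Pressing Fire pre-fills the timer for an immediate shot; RYogaFire is an uncalled right-gun variant.
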(event EventBeginPlay)

(event EventTick
  (params (DeltaSeconds :type Float%20%28single-precision%29))
  (CallFunction|Move DeltaSeconds)
  ;[0.15 0.15 0.15 0.5] 발사버튼을 눌렀다면
  (if (Variables|Default|GetIsFiring?)
    ;[0.15 0.15 0.15 0.5] 시간이 흐른다.
    (Variables|Default|SetCurrentTime (+ (Variables|Default|GetCurrentTime) (Utilities|Time|GetWorldDeltaSeconds)))
    ;[0.15 0.15 0.15 0.5] 생성시간이 됐다면
    (if (> (Variables|Default|GetCurrentTime) (Variables|Default|GetCreateTime))
      ;[0.15 0.15 0.15 0.5] 왼쪽 총알한발 발사
      (CallFunction|YogaFire (Variables|Default|GetLFirePosition))
      ;[0.15 0.15 0.15 0.5] 오른쪽 총알한발 발사
      (CallFunction|YogaFire (Variables|Default|GetRFirePosition))
      (Variables|Default|SetCurrentTime 0.0))))

(event Input|ActionEvents|InputActionFire
  (params (Key :type Key%20Structure :default "None"))
  (:Pressed
    (Variables|Default|SetIsFiring? true)
    (Variables|Default|SetCurrentTime (Variables|Default|GetCreateTime)))
  (:Released
    (Variables|Default|SetIsFiring? false)))

(event Input|AxisEvents|InputAxisHorizontal
  (params (AxisValue :type Float%20%28single-precision%29))
  ;[0.15 0.15 0.15 0.5] 방향이 필요하다.
  (Variables|Default|SetDirection (Math|Vector|MakeVector 0.0 AxisValue (stale Input|AxisEvents|InputAxisVertical AxisValue))))

(event Input|AxisEvents|InputAxisVertical
  (params (AxisValue :type Float%20%28single-precision%29))
  ;[0.15 0.15 0.15 0.5] 방향이 필요하다.
  (Variables|Default|SetDirection (Math|Vector|MakeVector 0.0 (stale Input|AxisEvents|InputAxisHorizontal AxisValue) AxisValue)))

(fn ConstructionScript)

(fn YogaFire
  (params (FirePosition :type Scene%20Component%20Object%20Reference))
  ;[0.15 0.15 0.15 0.5] 총알발사기능
  (Game|SpawnActorfromClass "/Game/Blueprints/BP_Bullet.BP_Bullet_C" (Math|Transform|MakeTransform (Transformation|GetWorldLocation FirePosition) "0, 0, 0" "1.000000,1.000000,1.000000") "Undefined" "MultiplyWithRoot" 0 0)
  (Audio|PlaySound2D "/Game/gun.gun" 1.0 1.0 0.0 0 0))

(fn Move
  (params (A :type Float%20%28single-precision%29))
  ;[0.15 0.15 0.15 0.5] 이동하고 싶다.
  (Transformation|SetActorLocation (+ (* A (* (Variables|Default|GetDirection) (Variables|Default|GetSpeed))) (Transformation|GetActorLocation)) false false))

(fn RYogaFire
  ;[0.15 0.15 0.15 0.5] 총알발사기능
  (Game|SpawnActorfromClass "/Game/Blueprints/BP_Bullet.BP_Bullet_C" (Math|Transform|MakeTransform (Transformation|GetWorldLocation (Variables|Default|GetRFirePosition)) "0, 0, 0" "1.000000,1.000000,1.000000") "Undefined" "MultiplyWithRoot" 0 0)
  (Audio|PlaySound2D "/Game/gun.gun" 1.0 1.0 0.0 0 0))